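; Manager actor that spawns bubbles and tower obstacles around its owner, likely the player character, as it moves.
; Each Tick rolls to spawn a randomly sized BouncingBubble in a box around the owner, then rarely a BP_Tower_Obstacle in a box offset along the manager's forward vector.
; A BP_KillBubbleActor spawned at BeginPlay is swept along at a fixed world-X offset behind the owner.
; Debug boxes show both spawn volumes.
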(event EventBeginPlay
  (Variables|Default|SetSpawnStartLocation (Components|GetOwner))
  (bind _returnvalue (Game|SpawnActorfromClass "/Game/Landscape/Systems/BP_KillBubbleActor.BP_KillBubbleActor_C" (Math|Conversions|ToTransform(Vector) (+ (Transformation|GetActorLocation (Components|GetOwner)) "-500.000000,0.000000,0.000000")) "Undefined" "MultiplyWithRoot" 0 0))
  (Variables|Default|SetCurrentBubbleKiller _returnvalue)
  (Variables|Default|SetReturn%20Value%20Z (.z (Transformation|GetActorLocation (Components|GetOwner)))))

(event EventTick
  (params (DeltaSeconds :type Float%20%28single-precision%29))
  (bind _returnvalue (Components|GetOwner))
  (bind _spawnplayerbound (Variables|Default|GetSpawnPlayerBound))
  (bind _spawnplayerbound_2 (Variables|Default|GetSpawnPlayerBound))
  (bind _returnvalue_2 (Transformation|GetActorLocation _returnvalue))
  (Transformation|SetRelativeLocation (Variables|/Script/Engine.Actor|GetRootComponent (Variables|Default|GetCurrentBubbleKiller)) (+ (Transformation|GetActorLocation (Components|GetOwner)) "-3000.000000,0.000000,0.000000") true false)
  (Utilities|IsValid (Components|GetOwner)
    (:Is%20Valid
      (bind _output_get (Variables|Default|SetGetCharCurrentPos (Math|Vector|MakeVector (.x _returnvalue_2) (.y _returnvalue_2) (.z _returnvalue_2))))
      (Rendering|Debug|DrawDebugBox _output_get _spawnplayerbound "(R=0.000000,G=0.871303,B=1.000000,A=1.000000)" "0, 0, 0" 0.0 19.0)
      (if (<= (Math|Random|RandomIntegerinRange 0 100) 50)
        (Game|SpawnActorfromClass "/Game/Blueprints/Obstacles/BouncingBubble.BouncingBubble_C" (Math|Conversions|ToTransform(Vector) (Math|Random|RandomPointinBoundingBox _output_get _spawnplayerbound)) "AdjustIfPossibleButDontSpawnIfColliding" "MultiplyWithRoot" 0 (Math|Random|RandomFloatinRange 1.0 5.0) 0)
        (Rendering|Debug|DrawDebugBox (+ (* (+ (Variables|Default|GetSpawnPlayerBound) "10000.000000,0.000000,0.000000") (Transformation|GetActorForwardVector)) (Variables|Default|GetGetCharCurrentPos)) _spawnplayerbound_2 "(R=1.000000,G=0.000000,B=0.196886,A=1.000000)" "0, 0, 0" 0.0 19.0)
        (if (>= (Math|Random|RandomIntegerinRange 0 100) 99)
          (Game|SpawnActorfromClass "/Game/Blueprints/Obstacles/BP_Tower_Obstacle.BP_Tower_Obstacle_C" (Math|Conversions|ToTransform(Vector) (Math|Random|RandomPointinBoundingBox (+ (* (+ (Variables|Default|GetSpawnPlayerBound) "10000.000000,0.000000,0.000000") (Transformation|GetActorForwardVector)) (Variables|Default|GetGetCharCurrentPos)) _spawnplayerbound_2)) "AdjustIfPossibleButDontSpawnIfColliding" "MultiplyWithRoot" 0 (Math|Random|RandomFloatinRange 1.0 1e+01) 0))))
    (:Is%20Not%20Valid
      (Utilities|String|LogString "NAAAH"))))

(fn ConstructionScript)