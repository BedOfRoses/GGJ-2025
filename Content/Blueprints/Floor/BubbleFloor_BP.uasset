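; BubbleFloor_BP is a hazard floor that hurts and bounces the bubble player on contact.
; When its Box overlaps a BubblePlayerCharacter_BP, it applies one point of damage through the PlayerHealthComponent.
; It then cuts the character's horizontal velocity to about a third, zeroes vertical velocity, and launches it upward with a fixed world-space X push.
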(event OnComponentBeginOverlap(Box)
  (params (OverlappedComponent :type Primitive%20Component%20Object%20Reference) (OtherActor :type Actor%20Object%20Reference) (OtherComp :type Primitive%20Component%20Object%20Reference) (OtherBodyIndex :type Integer) (bFromSweep :type Boolean) (SweepResult :type Hit%20Result%20Structure%20%28by%20ref%29))
  (if (Utilities|ClassIsChildOf (Utilities|GetClass OtherActor) "/Game/Blueprints/Characters/BubblePlayerCharacter_BP.BubblePlayerCharacter_BP_C")
    (Class|PlayerHealthComponent|ApplyDamage (Actor|GetComponentbyClass OtherActor "/Script/GGJ.PlayerHealthComponent") 1.0)
    (CallFunction|CasttoCharacterandLaunch OtherActor)))

(event EventBeginPlay)

(event Collision|EventActorBeginOverlap
  (params (OtherActor :type Actor%20Object%20Reference)))

(event EventTick
  (params (DeltaSeconds :type Float%20%28single-precision%29)))

(fn ConstructionScript)

(fn CasttoCharacterandLaunch
  (params (Object :type Object%20Object%20Reference))
  (bind _ascharacter (Utilities|Casting|CastToCharacter Object))
  (Variables|/Script/Engine.MovementComponent|SetVelocity (Variables|/Script/Engine.Character|GetCharacterMovement _ascharacter) (Math|Vector|MakeVector (* (.x (Variables|/Script/Engine.MovementComponent|GetVelocity (Variables|/Script/Engine.Character|GetCharacterMovement _ascharacter))) 0.333) (* (.y (Variables|/Script/Engine.MovementComponent|GetVelocity (Variables|/Script/Engine.Character|GetCharacterMovement _ascharacter))) 0.333) 0.0))
  (Character|LaunchCharacter _ascharacter "300.000000,0.000000,1000.000000" false false))