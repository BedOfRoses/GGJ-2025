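; BouncingBubble is an obstacle that launches the player character when it overlaps the bubble.
; On BeginPlay, SpawnSize sets the world scale of Sphere1.
; A Bubble overlap from BubblePlayerCharacter_BP zeroes vertical velocity, then adds a fixed world +X and upward launch divided by SpawnSize, so smaller bubbles launch harder.
; The bubble persists after a bounce because DestroyActor is unconnected, and a debug print remains.
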(event OnComponentBeginOverlap(Bubble)
  (params (OverlappedComponent :type Primitive%20Component%20Object%20Reference) (OtherActor :type Actor%20Object%20Reference) (OtherComp :type Primitive%20Component%20Object%20Reference) (OtherBodyIndex :type Integer) (bFromSweep :type Boolean) (SweepResult :type Hit%20Result%20Structure%20%28by%20ref%29))
  (if (Utilities|ClassIsChildOf (Utilities|GetClass OtherActor) "/Game/Blueprints/Characters/BubblePlayerCharacter_BP.BubblePlayerCharacter_BP_C")
    (Development|PrintString "OVERLAPP")
    (bind _ascharacter (Utilities|Casting|CastToCharacter OtherActor))
    (Variables|/Script/Engine.MovementComponent|SetVelocity (Variables|/Script/Engine.Character|GetCharacterMovement _ascharacter) (Math|Vector|MakeVector (.x (Variables|/Script/Engine.MovementComponent|GetVelocity (Variables|/Script/Engine.Character|GetCharacterMovement _ascharacter))) (.y (Variables|/Script/Engine.MovementComponent|GetVelocity (Variables|/Script/Engine.Character|GetCharacterMovement _ascharacter))) 0.0))
    (bind _output_get (Variables|Default|SetSizeToVelocity "1000.000000,0.000000,4000.000000"))
    (Character|LaunchCharacter _ascharacter (/ _output_get (Variables|Default|GetSpawnSize)) false false)))

(event EventBeginPlay
  (Transformation|SetWorldScale3D (Variables|Default|GetSphere1) (* (Variables|Default|GetSpawnSize) (Class|KismetMathLibrary|VectorOne))))

(event Collision|EventActorBeginOverlap
  (params (OtherActor :type Actor%20Object%20Reference)))

(event EventTick
  (params (DeltaSeconds :type Float%20%28single-precision%29)))

(fn ConstructionScript)